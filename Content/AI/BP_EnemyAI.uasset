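; Enemy AI character that chases the player on sight, punches in melee and dies when health runs out.
; Pawn sensing starts an AI MoveTo, then a punch montage and sphere overlap flag hits on Player-tagged actors.
; Damage, gated by a resettable DoOnce, and projectile hits share reaction and death montages before destruction.
; A freeze reaction blocks new chases until its montage completes, and Tick turns the health bar toward the camera.
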(event `self.ReceiveTick`
  (params (DeltaSeconds :type "Float (single-precision)"))
  (`|ExecutionSequence`
    (:`then_0`
      (if (not (`self.IsSeeingPlayer`))
        (`MovementComponent.StopMovementImmediately` (`self.CharacterMovement`))))
    (:`then_1`
      ;[1 1 1] Widget EnemyHealthBar
      (`SceneComponent.K2_SetWorldRotation` (`self.Widget`) (`KismetMathLibrary.FindLookAtRotation` (`SceneComponent.K2_GetComponentLocation` (`self.Widget`)) (`SceneComponent.K2_GetComponentLocation` (`PlayerCameraManager.TransformComponent` (`GameplayStatics.GetPlayerCameraManager` 0)))) false false))))

(event `self.PawnSensing.OnSeePawn`
  (params (Pawn :type "Pawn Object Reference"))
  (set `self.IsSeeingPlayer` true)
  (`self.FollowPlayer`))

(event `FollowPlayer`
  (if (not (`self.IsFreezed`))
    (set `self.CanAttack` true)
    (if (`self.IsSeeingPlayer`)
      (`|AIMoveTo` self (0.0 0.0 0.0) (`GameplayStatics.GetPlayerCharacter` 0) 70.0
        (:`OnSuccess`
          (if (`self.CanAttack`)
            (set `self.CanAttack` false)
            (if (not (<= (`self.Health`) 0.0))
              (`|PlayMontage` (`self.Mesh`) "/Game/Animations/SecondPunch_UE_Montage.SecondPunch_UE_Montage"
                (:`then`
                  (bind _outactors (`KismetSystemLibrary.SphereOverlapActors` (`SceneComponent.K2_GetComponentLocation` (`self.Arrow1`)) 100.0 (`self.Object Types`)))
                  (for _array_element _outactors
                    (if (`self.ActorHasTag` _array_element "Player")
                      (set `self.GettedDamage` true)))
                  (`KismetSystemLibrary.Delay` 2.5)
                  (set `self.CanAttack` true))
                (:`OnInterrupted`
                  (bind _returnvalue (`GameplayStatics.GetActorOfClass` "/Game/ThirdPerson/Blueprints/BP_ThirdPersonCharacter.BP_ThirdPersonCharacter_C"))
                  (bind _asbp_third_person_character (cast `/Game/ThirdPerson/Blueprints/BP_ThirdPersonCharacter` _returnvalue))
                  (`/Game/ThirdPerson/Blueprints/BP_ThirdPersonCharacter.ResetApplyDamage` _asbp_third_person_character)))))))
      (else
        (set `self.IsSeeingPlayer` false)))))

(event `Freeze Reaction`
  (params (InString :type String))
  (set `self.IsFreezed` true)
  (`KismetSystemLibrary.PrintString` "Hello")
  (`|PlayMontage` (`self.Mesh`) "/Game/Animations/FreezeReaction_UE_Montage.FreezeReaction_UE_Montage"
    (:`OnCompleted`
      (set `self.IsFreezed` false)
      (`KismetSystemLibrary.PrintString` "enemy"))))

(event `self.ReceiveAnyDamage`
  (params (Damage :type "Float (single-precision)") (DamageType :type "DamageType Object Reference") (InstigatedBy :type "Controller Object Reference") (DamageCauser :type "Actor Object Reference"))
  ;[1 1 1] ApplyingDamage
  (if (not (`SkeletalMeshComponent.IsPlaying` (`self.Mesh`)))
    (`/Engine/EditorBlueprintResources/StandardMacros.DoOnce` false :!label _label
      (:`Completed`
        (set `self.Health` (- (`self.Health`) Damage))
        (`KismetSystemLibrary.PrintString` (`KismetStringLibrary.Conv_DoubleToString` (`self.Health`)) :!label _label_2)
        (`|PlayMontage` (`self.Mesh`) "/Game/AI/Animations/StandingReactLargeFromRight_UE_Montage.StandingReactLargeFromRight_UE_Montage"
          (:`then`
            (if (<= (`self.Health`) 0.0)
              (`|PlayMontage` (`self.Mesh`) "/Game/AI/Animations/FallingBackDeath_UE_Montage.FallingBackDeath_UE_Montage"
                (:`then`
                  (`KismetSystemLibrary.Delay` 1.8)
                  (`self.K2_DestroyActor`))))))))))

(event `AttackEvent`
  ;[1 1 1] ApplyingDamage
  (goto _label :!via `Reset`))

(event `ProjectileHit`
  (params (Health :type "Float (double-precision)"))
  ;[1 1 1] ApplyingDamage
  (set `self.Health` (- (`self.Health`) Health))
  (goto _label_2))

(fn `UserConstructionScript`)
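; BP_Stan is a short-lived stun skill actor that immobilizes enemies overlapping it and destroys itself five seconds after spawning.
; On overlap, it ignores the player character, casts the other actor to BP_EnemyAI and disables its movement.
; A single three-second Delay precedes a debug print and restoring Walking mode, so overlaps during that delay or late in the actor's lifetime can leave enemies frozen.
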(event `self.ReceiveBeginPlay`
  (`KismetSystemLibrary.Delay` 5.0)
  (`self.K2_DestroyActor`))

(event `self.ReceiveActorBeginOverlap`
  (params (OtherActor :type "Actor Object Reference"))
  (bind _asbp_third_person_character (cast `/Game/ThirdPerson/Blueprints/BP_ThirdPersonCharacter` (`GameplayStatics.GetPlayerCharacter` 0)))
  (if (!= OtherActor _asbp_third_person_character)
    (bind _asbp_enemy_ai (cast `/Game/AI/BP_EnemyAI` OtherActor))
    (`CharacterMovementComponent.DisableMovement` (`Character.CharacterMovement` _asbp_enemy_ai))
    (`KismetSystemLibrary.Delay` 3.0)
    (`KismetSystemLibrary.PrintString` "Hello")
    (`CharacterMovementComponent.SetMovementMode` (`Character.CharacterMovement` _asbp_enemy_ai) "MOVE_Walking" 0)))

(fn `UserConstructionScript`)
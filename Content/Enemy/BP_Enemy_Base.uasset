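; Base enemy character Blueprint that provides attack, patrol route and movement speed functions.
; Attack plays a punch montage on the mesh and calls the OnAttackEnd dispatcher whether the montage completes or is interrupted.
; GetPatrolRoute returns the enemy's assigned route, and SetMovementSpeed maps a speed state from idle to sprinting onto the character's max walk speed.
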(event `Attack`
  (`|PlayMontage` (`self.Mesh`) "/Game/Animations/SecondPunch_UE_Montage.SecondPunch_UE_Montage"
    (:`OnCompleted`
      _)
    (:`OnInterrupted`
      _))
  (`self.OnAttackEnd`))

(fn `GetPatrolRoute`
  (returns (PatrolRoute :type "/Game/Enemy/AI/BP_PatrolRoute Object Reference"))
  (return (`self.PatrolRoute`)))

(fn `SetMovementSpeed`
  (params (Speed :type "/Game/Enemy/AI/Enums/E_MovementSpeed Enum" :default "NewEnumerator0"))
  (returns (SpeedValue :type "Float (double-precision)"))
  (set `CharacterMovementComponent.MaxWalkSpeed` (select `/Game/Enemy/AI/Enums/E_MovementSpeed` Speed :`NewEnumerator1` 100.0 :`NewEnumerator2` 300.0 :`NewEnumerator3` 500.0 :!type "Float (single-precision)") (`self.CharacterMovement`))
  (return 0.0))

(fn `UserConstructionScript`)